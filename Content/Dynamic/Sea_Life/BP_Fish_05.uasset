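; BP_Fish_05 is a sea-life fish pawn whose AI movement mixes fleeing from and following the player.
; BeginPlay starts both: RunAway repeatedly moves to random reachable points within 400 units, its intended away-from-player offset cancelled by Z-only scaling and flattening.
; FollowPlayer approaches within 1400 units, then after a random delay re-triggers both.
; SetMoveSpeed maps states to walk speeds but is not called here.
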(event `self.ReceiveBeginPlay`
  ;[1 1 1] Enemy Movement
  (`|ExecutionSequence` :!label _label
    (:`then_0`
      (bind _asbp_player (cast `/Game/Dynamic/Player/BP_Player` (`GameplayStatics.GetPlayerCharacter` 0)))
      (set `self.Character Ref` _asbp_player)
      (`self.Run Away`))
    (:`then_1`
      (`self.FollowPlayer`))))

(event `Run Away`
  (bind _returnvalue (`self.K2_GetActorLocation`))
  ;[1 1 1] Fish runaway
  (`|AIMoveTo` self (`NavigationSystemV1.K2_GetRandomReachablePointInRadius` (`KismetMathLibrary.MakeVector` (.x (+ _returnvalue (* (`KismetMathLibrary.GetForwardVector` (`KismetMathLibrary.FindLookAtRotation` _returnvalue (`self.K2_GetActorLocation` (`self.Character Ref`)))) (0.0 0.0 -500.0)))) (.y (+ _returnvalue (* (`KismetMathLibrary.GetForwardVector` (`KismetMathLibrary.FindLookAtRotation` _returnvalue (`self.K2_GetActorLocation` (`self.Character Ref`)))) (0.0 0.0 -500.0)))) (.z _returnvalue)) 400.0 null null) null
    (:`OnSuccess`
      _)
    (:`OnFail`
      _))
  (`self.Run Away`))

(event `FollowPlayer`
  ;[1 1 1] Enemy Movement
  (`|AIMoveTo` self (0.0 0.0 0.0) (`GameplayStatics.GetPlayerCharacter` 0) 1400.0
    (:`OnSuccess`
      (`KismetSystemLibrary.Delay` (`KismetMathLibrary.RandomFloatInRange` 0.3 (+ (`KismetMathLibrary.MultiplyByPi` (`KismetMathLibrary.RandomFloat`)) (`KismetMathLibrary.MultiplyMultiply_FloatFloat` 1.0 2.0))))
      (goto _label))))

(fn `GetPathRoute`
  (returns (PathRoute :type "/Game/Dynamic/Sea_Life/AI/BP_Fish_Movement_Patrol_Fish_01 Object Reference"))
  (return (`self.PathRoute`)))

(fn `SetMoveSpeed`
  (params (Speed :type "/Game/Dynamic/Sea_Life/AI/Enums/E_Movement_Speed Enum" :default "NewEnumerator0"))
  (returns (`Speed Value` :type "Float (double-precision)"))
  (bind _output_get (set `CharacterMovementComponent.MaxWalkSpeed` (select `/Game/Dynamic/Sea_Life/AI/Enums/E_Movement_Speed` Speed :`NewEnumerator0` 200.0 :`NewEnumerator1` 600.0 :`NewEnumerator2` 400.0 :`NewEnumerator3` 100.0 :!type "Float (single-precision)") (`self.CharacterMovement`)))
  (return _output_get))

(fn `UserConstructionScript`)