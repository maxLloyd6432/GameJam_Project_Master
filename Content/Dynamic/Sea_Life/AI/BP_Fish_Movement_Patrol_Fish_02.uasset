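; Fish patrol movement Blueprint that steps an index along a spline Path to provide patrol points for a sea-life fish.
; FishPathIncremental advances PathIndex by PathDirection and flips the direction at either end of the spline, producing a back-and-forth ping-pong route.
; GetSplinePointAsWorldPos returns the world-space location of the current spline point.
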(event `Fish Path Incremental`
  ;[0.4187 1 0.4793] Increment Function_StretchGoal - Multiple Path Following Routes
  (bind _output_get (set `self.PathIndex` (+ (`self.PathIndex`) (`self.PathDirection`))))
  (if (== _output_get (- (`SplineComponent.GetNumberOfSplinePoints` (`self.Path`)) 1))
    (set `self.PathDirection` -1)
    (elif (== (`self.PathIndex`) 0)
      (set `self.PathDirection` 1))))

(fn `Get Spline Point as World Pos`
  (returns (Location :type "Vector Structure"))
  ;[1 1 1] Increment Function_StretchGoal - Multiple Path Following Routes
  (return (`SplineComponent.GetLocationAtSplinePoint` (`self.Path`) (`self.PathIndex`) "World")))

(fn `UserConstructionScript`)