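; BP_Fish_02 is a sea-life fish that follows the player, labelled as enemy movement.
; From BeginPlay, FollowPlayer runs AI MoveTo toward the player character with a loose acceptance radius, repeating after a delay only on success.
; A stretch-goal stare event caches the BP_Player actor and opens a Tick-fed gate that yaws the fish toward it.
; Nothing in this graph calls that stare event.
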(event `self.ReceiveBeginPlay`
  ;[1 1 1] Enemy Movement
  (`self.FollowPlayer`))

(event `FollowPlayer`
  ;[1 1 1] Enemy Movement
  (`|AIMoveTo` self (0.0 0.0 0.0) (`GameplayStatics.GetPlayerCharacter` 0) 800.0
    (:`OnSuccess`
      (`KismetSystemLibrary.Delay` 5.0)
      (`self.FollowPlayer`))))

(event `CustomEvent`
  (bind (_returnvalue_roll _returnvalue_pitch _returnvalue_yaw) (`KismetMathLibrary.BreakRotator` (`KismetMathLibrary.FindLookAtRotation` (`self.K2_GetActorLocation`) (`self.K2_GetActorLocation` (`self.LookCharacter`)))))
  ;[1 1 1] Stretch Goal- BP_Fish_01-BP Stare Function
  (`|ExecutionSequence`
    (:`then_0`
      (bind _returnvalue (`GameplayStatics.GetActorOfClass` "/Game/Dynamic/Player/BP_Player.BP_Player_C"))
      (`/Engine/EditorBlueprintResources/StandardMacros.IsValid` _returnvalue
        (:`Is Valid`
          (set `self.LookCharacter` _returnvalue))))
    (:`then_1`
      (goto _label :!via `Open`))))

(event `self.ReceiveTick`
  (params (DeltaSeconds :type "Float (single-precision)"))
  (bind (_returnvalue_roll _returnvalue_pitch _returnvalue_yaw) (`KismetMathLibrary.BreakRotator` (`KismetMathLibrary.FindLookAtRotation` (`self.K2_GetActorLocation`) (`self.K2_GetActorLocation` (`self.LookCharacter`)))))
  ;[1 1 1] Stretch Goal- BP_Fish_01-BP Stare Function
  (`/Engine/EditorBlueprintResources/StandardMacros.Gate` true :!label _label
    (:`Exit`
      (`self.K2_SetActorRotation` (`KismetMathLibrary.MakeRotator` 0.0 0.0 _returnvalue_yaw)))))

(fn `UserConstructionScript`)