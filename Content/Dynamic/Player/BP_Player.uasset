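; Player boat Character that drives around, fires nets on a cooldown, collects fish and takes damage until destroyed.
; Input axes handle movement and turning, movement keys tilt the mesh and toggle spray, and holding Space changes speed and acceleration while locking turning.
; W, S and F emit noise or damage perception events.
; The HUD is created and stats reset in OnLanded, then updated on damage and fish pickup.
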(event `Key|LeftMouseButton`
  (params (Key :type "Key Structure"))
  ;[1 1 1] Fire Bullet
  (:`Pressed`
    (if (not (`self.Cooldown`))
      (`|SpawnActorFromClass` "/Game/Dynamic/Player/Net/Pawn_Net.Pawn_Net_C" (`SceneComponent.K2_GetComponentToWorld` (`self.Projectilespawn`)) "Undefined" "MultiplyWithRoot" null null)
      (set `self.Cooldown` true)
      (`KismetSystemLibrary.Delay` 0.8)
      (set `self.Cooldown` false)
      (`KismetSystemLibrary.PrintString` "CooldownOver"))))

(event `self.ReceiveBeginPlay`
  (`SceneComponent.SetHiddenInGame` (`self.RightSpray`) true false)
  (`SceneComponent.SetHiddenInGame` (`self.LeftSpray`) true false)
  (`SceneComponent.SetHiddenInGame` (`self.Middlespray`) true false)
  (`SceneComponent.SetHiddenInGame` (`self.Speedlines`) true false))

(event `Key|D`
  (params (Key :type "Key Structure"))
  ;[1 1 1] Jets
  (:`Pressed`
    (`SceneComponent.SetHiddenInGame` (`self.RightSpray`) false false)
    (`SceneComponent.K2_AddRelativeRotation` (`self.BoatMesh`) (struct :`Roll` -8.0) false false))
  (:`Released`
    (`SceneComponent.SetHiddenInGame` (`self.RightSpray`) true false)
    (`SceneComponent.K2_AddRelativeRotation` (`self.BoatMesh`) (struct :`Roll` 8.0) false false)))

(event `InputAxis|Forward`
  (params (AxisValue :type "Float (single-precision)"))
  (`self.AddMovementInput` (`self.GetActorForwardVector`) AxisValue))

(event `Key|A`
  (params (Key :type "Key Structure"))
  ;[1 1 1] Jets
  (:`Pressed`
    (`SceneComponent.SetHiddenInGame` (`self.LeftSpray`) false false)
    (`SceneComponent.K2_AddRelativeRotation` (`self.BoatMesh`) (struct :`Roll` 8.0) false false))
  (:`Released`
    (`SceneComponent.SetHiddenInGame` (`self.LeftSpray`) true false)
    (`SceneComponent.K2_AddRelativeRotation` (`self.BoatMesh`) (struct :`Roll` -8.0) false false)))

(event `InputAxis|TurnLeft`
  (params (AxisValue :type "Float (single-precision)"))
  ;[1 1 1] Turn
  (if (not (`self.Speeding`))
    (`self.AddControllerYawInput` (* AxisValue (`self.Turnspeed`)))))

(event `Key|W`
  (params (Key :type "Key Structure"))
  ;[1 1 1] Jets
  (:`Pressed`
    (`SceneComponent.K2_AddRelativeRotation` (`self.BoatMesh`) (struct :`Pitch` -10.0) false false)
    (`SceneComponent.SetHiddenInGame` (`self.Middlespray`) false false))
  (:`Released`
    (`SceneComponent.K2_AddRelativeRotation` (`self.BoatMesh`) (struct :`Pitch` 10.0) false false)
    (`SceneComponent.SetHiddenInGame` (`self.Middlespray`) true false)))

(event `InputAxis|TurnRight`
  (params (AxisValue :type "Float (single-precision)"))
  ;[1 1 1] Turn
  (if (not (`self.Speeding`))
    (`self.AddControllerYawInput` (* AxisValue (`self.Turnspeed`)))))

(event `Key|SpaceBar`
  (params (Key :type "Key Structure"))
  ;[1 1 1] Speeding
  (:`Pressed`
    (`SceneComponent.SetHiddenInGame` (`self.Speedlines`) false false)
    (set `self.Speeding` true)
    (set `CharacterMovementComponent.MaxAcceleration` 700.0 (`self.CharacterMovement`))
    (set `CharacterMovementComponent.MaxWalkSpeed` (`self.WalkSpeed`) (`self.CharacterMovement`))
    (`KismetSystemLibrary.PrintString` "speedingon"))
  (:`Released`
    (`SceneComponent.SetHiddenInGame` (`self.Speedlines`) true false)
    (set `self.Speeding` false)
    (set `CharacterMovementComponent.MaxAcceleration` 300.0 (`self.CharacterMovement`))
    (set `CharacterMovementComponent.MaxWalkSpeed` (`self.BoostSpeed`) (`self.CharacterMovement`))
    (`KismetSystemLibrary.PrintString` "speedingoff")))

(event `Key|W`
  (params (Key :type "Key Structure"))
  (bind _returnvalue (`self.K2_GetActorLocation`))
  ;[0.6122 0.1448 1] Emit Noise/Particle
  (:`Pressed`
    (`self.MakeNoise` 1.0 self _returnvalue)
    (`AISense_Hearing.ReportNoiseEvent` _returnvalue 1.0 null)
    ;;[1 0 0.01345] Problem - Auto Destroy not working
    (`GameplayStatics.SpawnEmitterAtLocation` (`self.Emitter Template`) _returnvalue)
    (`GameplayStatics.PlaySoundAtLocation` "/Game/Static/Audio/Boat_Engine_sandermotions.Boat_Engine_sandermotions" _returnvalue (struct) 1.0 1.0 0.0 null null null null)))

(event `Key|S`
  (params (Key :type "Key Structure"))
  (bind _returnvalue (`self.K2_GetActorLocation`))
  ;[0.6122 0.1448 1] Emit Noise/Particle
  (:`Pressed`
    (`self.MakeNoise` 1.0 self _returnvalue)
    ;;[1 0 0.01345] Problem - Auto Destroy not working
    (`GameplayStatics.SpawnEmitterAtLocation` (`self.Emitter Template`) _returnvalue)
    (`GameplayStatics.PlaySoundAtLocation` "/Game/Static/Audio/Boat_Engine_sandermotions.Boat_Engine_sandermotions" _returnvalue (struct) 1.0 1.0 0.0 null null null null)))

(event `Key|F`
  (params (Key :type "Key Structure"))
  (:`Pressed`
    (bind _returnvalue (`GameplayStatics.GetActorOfClass` "BP_Player_C"))
    (`AISense_Damage.ReportDamageEvent` _returnvalue self 1.0 (`self.K2_GetActorLocation`))))

(event `self.OnLanded`
  (params (Hit :type "HitResult Structure (by ref)"))
  ;[0.2016 0.9741 1] UI
  (bind _returnvalue (`|CreateWidget` "/Game/UI/Widgets/WB_GameUI.WB_GameUI_C"))
  (bind _output_get (set `self.Game UI` _returnvalue))
  (`UserWidget.AddToViewport` _output_get 0)
  (set `self.CurrentHealth` (`self.MaxHealth`))
  (set `self.CollectedFish` 0))

(event `self.ReceiveAnyDamage`
  (params (Damage :type "Float (single-precision)") (DamageType :type "DamageType Object Reference") (InstigatedBy :type "Controller Object Reference") (DamageCauser :type "Actor Object Reference"))
  (bind _maxhealth (`self.MaxHealth`))
  (bind _currenthealth (`self.CurrentHealth`))
  ;[0.2016 0.9741 1] UI
  (bind _output_get (set `self.CurrentHealth` (`KismetMathLibrary.FClamp` (- _currenthealth Damage) 0.0 _maxhealth)))
  (`/Game/UI/Widgets/WB_GameUI.Update Health UI` (`self.Game UI`) _output_get _maxhealth)
  (if (== _currenthealth 0.0)
    (`self.K2_DestroyActor`)
    (`/Game/UI/Widgets/WB_GameUI.Game Over` (`self.Game UI`))))

(event `Fish Collected`
  ;[0.2016 0.9741 1] UI
  (bind _output_get (set `self.CollectedFish` (+ 1 (`self.CollectedFish`))))
  (`/Game/UI/Widgets/WB_GameUI.Update Fish UI` (`self.Game UI`) _output_get))

(fn `UserConstructionScript`)